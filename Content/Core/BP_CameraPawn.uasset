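; Camera pawn that the player flies around the level with the keyboard.
; BeginPlay places it at a fixed elevated starting location and pitch.
; Tick polls WASD for horizontal movement and E/Q for up and down, shifting the actor along world axes in fixed steps.
; Movement is not scaled by delta time, so speed depends on frame rate, and a mouse position lookup is left unused.
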(event EventBeginPlay
  (Transformation|SetActorLocationAndRotation (Math|Vector|MakeVector -7.6e+02 -6e+01 1.82e+03) (Math|Rotator|MakeRotator 0.0 2e+01 0.0)))

(event EventTick
  (params (DeltaSeconds :type Float%20%28single-precision%29))
  (bind _returnvalue (Transformation|GetActorLocation))
  (bind _returnvalue_2 (Transformation|GetActorLocation))
  (bind _returnvalue_3 (Transformation|GetActorLocation))
  (bind _returnvalue_4 (Transformation|GetActorLocation))
  (bind _returnvalue_5 (Transformation|GetActorLocation))
  (bind _returnvalue_6 (Transformation|GetActorLocation))
  ;[1 1 1] Move Camera Right
  (Utilities|FlowControl|Sequence
    (:then_0
      (if (Game|Player|IsInputKeyDown (Game|GetPlayerController 0) "D")
        (Transformation|SetActorLocation (Math|Vector|MakeVector (.x _returnvalue) (+ (.y _returnvalue) 2e+01) (.z _returnvalue)) false false)))
    (:then_1
      (if (Game|Player|IsInputKeyDown (Game|GetPlayerController 0) "A")
        (Transformation|SetActorLocation (Math|Vector|MakeVector (.x _returnvalue_2) (- (.y _returnvalue_2) 2e+01) (.z _returnvalue_2)) false false)))
    (:then_2
      (if (Game|Player|IsInputKeyDown (Game|GetPlayerController 0) "W")
        (Transformation|SetActorLocation (Math|Vector|MakeVector (+ (.x _returnvalue_4) 2e+01) (.y _returnvalue_4) (.z _returnvalue_4)) false false)))
    (:then_3
      (if (Game|Player|IsInputKeyDown (Game|GetPlayerController 0) "S")
        (Transformation|SetActorLocation (Math|Vector|MakeVector (- (.x _returnvalue_6) 2e+01) (.y _returnvalue_6) (.z _returnvalue_6)) false false)))
    (:then_4
      (if (Game|Player|IsInputKeyDown (Game|GetPlayerController 0) "E")
        (Transformation|SetActorLocation (Math|Vector|MakeVector (.x _returnvalue_5) (.y _returnvalue_5) (+ (.z _returnvalue_5) 2e+01)) false false)))
    (:then_5
      (if (Game|Player|IsInputKeyDown (Game|GetPlayerController 0) "Q")
        (Transformation|SetActorLocation (Math|Vector|MakeVector (.x _returnvalue_3) (.y _returnvalue_3) (- (.z _returnvalue_3) 2e+01)) false false)))))

(fn ConstructionScript)