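; Tower game control Blueprint that runs the money economy and handles cancelling build mode.
; On BeginPlay it adds a money widget to the viewport and starts a looping timer that increments money every second.
; The money total is read and written directly on the widget.
; Right mouse press calls CallCancelBuildMode and clears the build-mode flag.
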(event Custom|AddMoney
  (bind _widgetmoneyref (Variables|Default|GetWidgetMoneyRef))
  ;[1 1 1] Create the money widget, add money to it at intervals
  (Variables|/Game/Interface/Widget_Money.Widget_Money_C|SetMoney_MoneyWidget _widgetmoneyref (+ (Variables|/Game/Interface/Widget_Money.Widget_Money_C|GetMoney_MoneyWidget _widgetmoneyref) 1)))

(event EventBeginPlay
  ;[1 1 1] Create the money widget, add money to it at intervals
  (bind _returnvalue (UserInterface|CreateWidget "/Game/Interface/Widget_Money.Widget_Money_C"))
  (bind _output_get (Variables|Default|SetWidgetMoneyRef _returnvalue))
  (UserInterface|Viewport|AddtoViewport _output_get 0)
  (Utilities|Time|SetTimerbyEvent (delegate Custom|AddMoney) 1.0 true))

(event Input|MouseEvents|RightMouseButton
  (params (Key :type Key%20Structure :default "None"))
  ;[1 1 1] Cancel building mode
  (:Pressed
    (Default|CallCancelBuildMode)
    (Variables|Default|SetBuildModeActive false)))

(fn ConstructionScript)