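; BP_StandardTower is a tower that automatically fires at overlapping BP_EnemyMaster actors.
; A looping 1.5-second timer started on BeginPlay passes those overlaps to GetClosestTarget, then spawns a BP_NormalProjectile at the tower's transform with the result as TargetEnemy.
; Despite its name, GetClosestTarget keeps the farthest actor, because it replaces the candidate when the new distance is larger.
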(event Custom|FireStandard
  (bind _targets (CallFunction|GetClosestTarget (Collision|GetOverlappingActors "/Game/Blueprints/BP_EnemyMaster.BP_EnemyMaster_C" :!class /Script/Engine.Actor)))
  (bind _asbp_enemy_master (Utilities|Casting|CastToBP_EnemyMaster _targets))
  (Game|SpawnActorfromClass "/Game/Blueprints/BP_NormalProjectile.BP_NormalProjectile_C" (Transformation|GetActorTransform) "AlwaysSpawn" 0 _asbp_enemy_master 0))

(event EventBeginPlay
  (Utilities|Time|SetTimerbyEvent (delegate Custom|FireStandard) 1.5 true))

(fn ConstructionScript)

(fn GetClosestTarget
  (params (List :type Array%20of%20Actor%20Object%20References))
  (for _array_element List
    (LocalVariables|GetTempTarget
      (:then
        (if (< (LocalVariables|GetTempDistance) (Math|Vector|VectorLength (- (Transformation|GetActorLocation) (Transformation|GetActorLocation _array_element))))
          (LocalVariables|SetTempTarget _array_element)
          (LocalVariables|SetTempDistance (Math|Vector|VectorLength (- (Transformation|GetActorLocation) (Transformation|GetActorLocation _array_element))))))
      (:else
        (LocalVariables|SetTempTarget _array_element)
        (LocalVariables|SetTempDistance (Math|Vector|VectorLength (- (Transformation|GetActorLocation) (Transformation|GetActorLocation _array_element)))))))
  (return (LocalVariables|GetTempTarget)))