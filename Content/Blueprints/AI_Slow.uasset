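; AI_Slow is a destructible actor, by its name a slow AI, that takes damage from normal projectiles.
; Overlapping a BP_NormalProjectile destroys the projectile and removes one Health, and the actor destroys itself when Health reaches exactly zero.
; On BeginPlay it replaces its actor Tags with the value of its Tag variable.
; No movement or decision logic is defined in its graphs.
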(event Collision|EventActorBeginOverlap
  (params (OtherActor :type Actor%20Object%20Reference))
  (bind _asbp_normal_projectile (Utilities|Casting|CastToBP_NormalProjectile OtherActor))
  (Actor|DestroyActor _asbp_normal_projectile)
  (Variables|Default|SetHealth (- (Variables|Default|GetHealth) 1))
  (if (== (Variables|Default|GetHealth) 0)
    (Actor|DestroyActor)))

(event EventBeginPlay
  (Variables|Default|SetTags (Utilities|Array|MakeArray (Variables|Default|Gettag))))

(fn ConstructionScript)