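; Wave spawner actor that runs five timed enemy waves at its own location and drives the wave countdown widget.
; A one-second timer counts down, pauses while a wave runs, then resets and resumes.
; Each wave adds looping spawn timers for standard, fast and, from wave two, brute enemies, gated on a zero countdown.
; These timers are never cleared, so spawns stack until the last wave shows completion text and destroys the spawner.
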(event Custom|SpawnSlowEnemy3
  ;[1 1 1] Wave 3
  (if (== (Variables|Default|GetUntilNextWave) 0)
    (AI|SpawnAIFromClass "/Game/Blueprints/Enemies/BP_EnemyStandard.BP_EnemyStandard_C" 0 (Transformation|GetActorLocation) "0, 0, 0" false 0)))

(event Custom|SpawnBruteEnemy5
  ;[1 1 1] Wave 5
  (if (== (Variables|Default|GetUntilNextWave) 0)
    (AI|SpawnAIFromClass "/Game/Blueprints/Enemies/BP_EnemyBrute.BP_EnemyBrute_C" 0 (Transformation|GetActorLocation) "0, 0, 0" false 0)))

(event Custom|SpawnSlowEnemy4
  ;[1 1 1] Wave 4
  (if (== (Variables|Default|GetUntilNextWave) 0)
    (AI|SpawnAIFromClass "/Game/Blueprints/Enemies/BP_EnemyStandard.BP_EnemyStandard_C" 0 (Transformation|GetActorLocation) "0, 0, 0" false 0)))

(event Custom|SpawnFastEnemy4
  ;[1 1 1] Wave 4
  (if (== (Variables|Default|GetUntilNextWave) 0)
    (AI|SpawnAIFromClass "/Game/Blueprints/Enemies/BP_EnemyFast.BP_EnemyFast_C" 0 (Transformation|GetActorLocation) "0, 0, 0" false 0)))

(event Custom|Wave4
  ;[1 1 1] Wave 4
  (Utilities|Time|SetTimerbyEvent (delegate Custom|SpawnSlowEnemy4) 2.0 true)
  (Utilities|Time|SetTimerbyEvent (delegate Custom|SpawnFastEnemy4) 5.0 true)
  (Utilities|Time|SetTimerbyEvent (delegate Custom|SpawnBruteEnemy4) 1e+01 true))

(event Custom|SpawnBruteEnemy4
  ;[1 1 1] Wave 4
  (if (== (Variables|Default|GetUntilNextWave) 0)
    (AI|SpawnAIFromClass "/Game/Blueprints/Enemies/BP_EnemyBrute.BP_EnemyBrute_C" 0 (Transformation|GetActorLocation) "0, 0, 0" false 0)))

(event Custom|CountUntilNextWave
  (bind _widgetwavereference (Variables|Default|GetWidgetWaveReference))
  ;[1 1 1] Creates the wave widget, and controls the timer for waves, and triggers the waves accordingly. Triggers game over when the last wave is done.
  (bind _output_get (Variables|Default|SetUntilNextWave (- (Variables|Default|GetUntilNextWave) 1)))
  (Rendering|Components|TextRender|SetText (Variables|/Game/Interface/Widget_Wave.Widget_Wave_C|GetCountdownTilNextWave (stale EventBeginPlay _output_get)) (Utilities|Text|ToText(Integer) _output_get))
  (if (== (Variables|Default|GetUntilNextWave) 0)
    (Class|KismetSystemLibrary|PauseTimer 0 "CountUntilNextWave")
    (Appearance|SetColorandOpacity (Variables|/Game/Interface/Widget_Wave.Widget_Wave_C|GetCountdownTilNextWave (Variables|Default|GetWidgetWaveReference)) (Utilities|Struct|MakeSlateColor "(R=1.000000,G=0.000000,B=0.048397,A=1.000000)") :!class /Script/UMG.TextBlock)
    (bind _output_get_2 (Variables|Default|SetWhichWaveToTrigger (+ (Variables|Default|GetWhichWaveToTrigger) 1)))
    (Rendering|Components|TextRender|SetText (Variables|/Game/Interface/Widget_Wave.Widget_Wave_C|GetWaveNumber (Variables|Default|GetWidgetWaveReference)) (Utilities|Text|ToText(Integer) _output_get_2))
    (Utilities|FlowControl|Sequence
      (:then_0
        (if (== (Variables|Default|GetWhichWaveToTrigger) 1)
          (CallFunction|Wave1)
          (Utilities|FlowControl|Delay 3e+01 :!label _label)
          (Variables|Default|SetUntilNextWave 30)
          (Appearance|SetColorandOpacity (Variables|/Game/Interface/Widget_Wave.Widget_Wave_C|GetCountdownTilNextWave (Variables|Default|GetWidgetWaveReference)) (Utilities|Struct|MakeSlateColor "(R=0.000000,G=1.000000,B=0.031219,A=1.000000)") :!class /Script/UMG.TextBlock)
          (if (== (Variables|Default|GetWhichWaveToTrigger) 5)
            (Class|TextBlock|SetOpacity (Variables|/Game/Interface/Widget_Wave.Widget_Wave_C|GetCompletedText _widgetwavereference) 1.0)
            (Class|TextBlock|SetOpacity (Variables|/Game/Interface/Widget_Wave.Widget_Wave_C|GetTextWhichWave _widgetwavereference) 0.0)
            (Class|TextBlock|SetOpacity (Variables|/Game/Interface/Widget_Wave.Widget_Wave_C|GetWaveNumber _widgetwavereference) 0.0)
            (Actor|DestroyActor)
            (else
              (Class|KismetSystemLibrary|UnPauseTimer 0 "CountUntilNextWave")))))
      (:then_1
        (if (== (Variables|Default|GetWhichWaveToTrigger) 2)
          (CallFunction|Wave2)
          (goto _label)))
      (:then_2
        (if (== (Variables|Default|GetWhichWaveToTrigger) 3)
          (CallFunction|Wave3)
          (goto _label)))
      (:then_3
        (if (== (Variables|Default|GetWhichWaveToTrigger) 4)
          (CallFunction|Wave4)
          (goto _label)))
      (:then_4
        (if (== (Variables|Default|GetWhichWaveToTrigger) 5)
          (CallFunction|Wave5)
          (goto _label)))
      (:then_5
        (goto _label)))))

(event Custom|SpawnSlowEnemy5
  ;[1 1 1] Wave 5
  (if (== (Variables|Default|GetUntilNextWave) 0)
    (AI|SpawnAIFromClass "/Game/Blueprints/Enemies/BP_EnemyStandard.BP_EnemyStandard_C" 0 (Transformation|GetActorLocation) "0, 0, 0" false 0)))

(event Custom|SpawnSlowEnemy1
  ;[1 1 1] Wave 1
  (if (== (Variables|Default|GetUntilNextWave) 0)
    (AI|SpawnAIFromClass "/Game/Blueprints/Enemies/BP_EnemyStandard.BP_EnemyStandard_C" 0 (Transformation|GetActorLocation) "0, 0, 0" false 0)))

(event Custom|SpawnFastEnemy1
  ;[1 1 1] Wave 1
  (if (== (Variables|Default|GetUntilNextWave) 0)
    (AI|SpawnAIFromClass "/Game/Blueprints/Enemies/BP_EnemyFast.BP_EnemyFast_C" 0 (Transformation|GetActorLocation) "0, 0, 0" false 0)))

(event Custom|Wave1
  ;[1 1 1] Wave 1
  (Utilities|Time|SetTimerbyEvent (delegate Custom|SpawnSlowEnemy1) 2.0 true)
  (Utilities|Time|SetTimerbyEvent (delegate Custom|SpawnFastEnemy1) 5.0 true))

(event Custom|SpawnFastEnemy5
  ;[1 1 1] Wave 5
  (if (== (Variables|Default|GetUntilNextWave) 0)
    (AI|SpawnAIFromClass "/Game/Blueprints/Enemies/BP_EnemyFast.BP_EnemyFast_C" 0 (Transformation|GetActorLocation) "0, 0, 0" false 0)))

(event Custom|SpawnFastEnemy3
  ;[1 1 1] Wave 3
  (if (== (Variables|Default|GetUntilNextWave) 0)
    (AI|SpawnAIFromClass "/Game/Blueprints/Enemies/BP_EnemyFast.BP_EnemyFast_C" 0 (Transformation|GetActorLocation) "0, 0, 0" false 0)))

(event Custom|SpawnSlowEnemy2
  ;[1 1 1] Wave 2
  (if (== (Variables|Default|GetUntilNextWave) 0)
    (AI|SpawnAIFromClass "/Game/Blueprints/Enemies/BP_EnemyStandard.BP_EnemyStandard_C" 0 (Transformation|GetActorLocation) "0, 0, 0" false 0)))

(event Custom|SpawnFastEnemy2
  ;[1 1 1] Wave 2
  (if (== (Variables|Default|GetUntilNextWave) 0)
    (AI|SpawnAIFromClass "/Game/Blueprints/Enemies/BP_EnemyFast.BP_EnemyFast_C" 0 (Transformation|GetActorLocation) "0, 0, 0" false 0)))

(event Custom|Wave2
  ;[1 1 1] Wave 2
  (Utilities|Time|SetTimerbyEvent (delegate Custom|SpawnSlowEnemy2) 2.0 true)
  (Utilities|Time|SetTimerbyEvent (delegate Custom|SpawnFastEnemy2) 5.0 true)
  (Utilities|Time|SetTimerbyEvent (delegate Custom|SpawnBruteEnemy2) 1e+01 true))

(event Custom|SpawnBruteEnemy2
  ;[1 1 1] Wave 2
  (if (== (Variables|Default|GetUntilNextWave) 0)
    (AI|SpawnAIFromClass "/Game/Blueprints/Enemies/BP_EnemyBrute.BP_EnemyBrute_C" 0 (Transformation|GetActorLocation) "0, 0, 0" false 0)))

(event Custom|Wave5
  ;[1 1 1] Wave 5
  (Utilities|Time|SetTimerbyEvent (delegate Custom|SpawnSlowEnemy5) 2.0 true)
  (Utilities|Time|SetTimerbyEvent (delegate Custom|SpawnFastEnemy5) 5.0 true)
  (Utilities|Time|SetTimerbyEvent (delegate Custom|SpawnBruteEnemy5) 1e+01 true))

(event Custom|Wave3
  ;[1 1 1] Wave 3
  (Utilities|Time|SetTimerbyEvent (delegate Custom|SpawnSlowEnemy3) 2.0 true)
  (Utilities|Time|SetTimerbyEvent (delegate Custom|SpawnFastEnemy3) 5.0 true)
  (Utilities|Time|SetTimerbyEvent (delegate Custom|SpawnBruteEnemy3) 1e+01 true))

(event Custom|SpawnBruteEnemy3
  ;[1 1 1] Wave 3
  (if (== (Variables|Default|GetUntilNextWave) 0)
    (AI|SpawnAIFromClass "/Game/Blueprints/Enemies/BP_EnemyBrute.BP_EnemyBrute_C" 0 (Transformation|GetActorLocation) "0, 0, 0" false 0)))

(event EventBeginPlay
  ;[1 1 1] Creates the wave widget, and controls the timer for waves, and triggers the waves accordingly. Triggers game over when the last wave is done.
  (bind _returnvalue (UserInterface|CreateWidget "/Game/Interface/Widget_Wave.Widget_Wave_C"))
  (bind _output_get (Variables|Default|SetWidgetWaveReference _returnvalue))
  (UserInterface|Viewport|AddtoViewport _output_get 0)
  (Utilities|Time|SetTimerbyEvent (delegate Custom|CountUntilNextWave) 1.0 true))

(fn ConstructionScript)