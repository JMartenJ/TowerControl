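; BP_EnemyBrute is the Brute enemy, which takes damage from the radial tower's explosion.
; On BeginPlay it loads health, speed and strength from the enemy data table and reads the Radial row of the tower table.
; A looping half-second timer polls for overlap with the first BP_RadialExplosion found, subtracts that tower's damage from health and runs a death check.
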(event Custom|RadialHitBrute
  ;[1 1 1] Gives it damage from the radial tower explosion
  (bind _returnvalue (Actor|GetActorOfClass "/Game/Blueprints/Towers/BP_RadialExplosion.BP_RadialExplosion_C"))
  (if (Collision|IsOverlappingActor _returnvalue :!class /Script/Engine.Actor)
    (Variables|Default|SetHealth (- (Variables|Default|GetHealth) (.damage (stale EventBeginPlay _returnvalue_2))))
    (CallFunction|CheckIsDead)))

(event EventBeginPlay
  ;[1 1 1] Sets the stats for the enemy
  (bind _returnvalue (Utilities|GetDataTableRow "/Game/Blueprints/Enemies/EnemyDataTable.EnemyDataTable" "Brute")
    (:then
      (Variables|Default|SetHealth (.health _returnvalue))
      (Variables|/Script/Engine.CharacterMovementComponent|SetMaxWalkSpeed (Variables|Character|GetCharacterMovement) (.speed _returnvalue))
      (Variables|Default|SetStrenght (.strenght _returnvalue))
      ;[1 1 1] Gives it damage from the radial tower explosion
      (bind _returnvalue_2 (Utilities|GetDataTableRow "/Game/Blueprints/Towers/TowerData.TowerData" "Radial")
        (:then
          (Utilities|Time|SetTimerbyEvent (delegate Custom|RadialHitBrute) 0.5 true))))))

(fn ConstructionScript
  (|CallParentFunction))