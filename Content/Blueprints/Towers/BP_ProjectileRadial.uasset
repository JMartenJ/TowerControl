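; BP_ProjectileRadial is a tower projectile that spawns a BP_RadialExplosion and destroys itself when it overlaps an actor tagged "enemy".
; BeginPlay snapshots the target enemy's location, and Tick moves toward that fixed point at constant speed without homing.
; Speed comes from the TowerData "Radial" row, which is only looked up in the overlap event.
; A Delay in Tick destroys the projectile after about three seconds.
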(event Collision|EventActorBeginOverlap
  (params (OtherActor :type Actor%20Object%20Reference))
  ;[1 1 1] Flies towards its last known location, and creates an explosion when it hits an enemy
  (bind _returnvalue (Utilities|GetDataTableRow "/Game/Blueprints/Towers/TowerData.TowerData" "Radial")
    (:then
      (if (Actor|ActorHasTag OtherActor "enemy")
        (Game|SpawnActorfromClass "/Game/Blueprints/Towers/BP_RadialExplosion.BP_RadialExplosion_C" (Math|Conversions|ToTransform(Vector) (Transformation|GetActorLocation)) "Undefined" 0 0)
        (Actor|DestroyActor)))))

(event EventBeginPlay
  ;[1 1 1] Flies towards its last known location, and creates an explosion when it hits an enemy
  (Variables|Default|SetLastKnownLocation (Transformation|GetActorLocation (Variables|Default|GetTargetEnemy))))

(event EventTick
  (params (DeltaSeconds :type Float%20%28single-precision%29))
  ;[1 1 1] Flies towards its last known location, and creates an explosion when it hits an enemy
  (Transformation|SetActorLocation (Math|Interpolation|VInterptoConstant (Transformation|GetActorLocation) (Variables|Default|GetLastKnownLocation) DeltaSeconds (.projectilespeed (stale Collision|EventActorBeginOverlap _returnvalue))) false false)
  (Utilities|FlowControl|Delay 3.0)
  (Actor|DestroyActor))

(fn ConstructionScript)