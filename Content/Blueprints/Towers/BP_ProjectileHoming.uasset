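; Homing tower projectile that chases its target enemy and damages the enemy it overlaps.
; Tick moves it toward TargetEnemy at constant speed, using ProjectileSpeed from the "Homing" TowerData row that is looked up only in the overlap event.
; On overlapping a BP_EnemyMaster, it subtracts the row's Damage from Health, destroys itself and calls CheckIsDead.
; A Delay in Tick also destroys it after five seconds.
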(event Collision|EventActorBeginOverlap
  (params (OtherActor :type Actor%20Object%20Reference))
  ;[1 1 1] Deals damage to enemies, and searches for its target
  (bind _returnvalue (Utilities|GetDataTableRow "/Game/Blueprints/Towers/TowerData.TowerData" "Homing")
    (:then
      (bind _asbp_enemy_master (Utilities|Casting|CastToBP_EnemyMaster OtherActor))
      (Variables|/Game/Blueprints/Enemies/BP_EnemyMaster.BP_EnemyMaster_C|SetHealth _asbp_enemy_master (- (Variables|/Game/Blueprints/Enemies/BP_EnemyMaster.BP_EnemyMaster_C|GetHealth _asbp_enemy_master) (.damage _returnvalue)))
      (Actor|DestroyActor)
      (Default|CheckIsDead _asbp_enemy_master))))

(event EventTick
  (params (DeltaSeconds :type Float%20%28single-precision%29))
  ;[1 1 1] Deals damage to enemies, and searches for its target
  (Transformation|SetActorLocation (Math|Interpolation|VInterptoConstant (Transformation|GetActorLocation) (Transformation|GetActorLocation (Variables|Default|GetTargetEnemy)) DeltaSeconds (.projectilespeed (stale Collision|EventActorBeginOverlap _returnvalue))) false false)
  (Utilities|FlowControl|Delay 5.0)
  (Actor|DestroyActor))

(fn ConstructionScript)