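; Radial tower that periodically spawns a radial projectile at itself when an enemy overlaps it.
; On BeginPlay it reads the "Radial" TowerData row to set the sphere radius (range) and a looping fire timer.
; Each tick of that timer passes overlapping enemies to GetClosestTarget and hands the result to the projectile as TargetEnemy.
; Despite its name, GetClosestTarget's comparison keeps the farthest enemy.
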(event Custom|FireRadial
  ;[1 1 1] Fire a radial projectile
  (bind _targets (CallFunction|GetClosestTarget (Collision|GetOverlappingActors "/Game/Blueprints/Enemies/BP_EnemyMaster.BP_EnemyMaster_C" :!class /Script/Engine.Actor)))
  (bind _asbp_enemy_master (Utilities|Casting|CastToBP_EnemyMaster _targets))
  (Game|SpawnActorfromClass "/Game/Blueprints/Towers/BP_ProjectileRadial.BP_ProjectileRadial_C" (Transformation|GetActorTransform) "AlwaysSpawn" 0 _asbp_enemy_master 0))

(event EventBeginPlay
  ;[1 1 1] Fire a radial projectile
  (bind _returnvalue (Utilities|GetDataTableRow "/Game/Blueprints/Towers/TowerData.TowerData" "Radial")
    (:then
      (Components|Sphere|SetSphereRadius (Variables|Default|GetSphere) (.range _returnvalue) true)
      (Utilities|Time|SetTimerbyFunctionName 0 "FireRadial" (.firerate _returnvalue) true))))

(fn ConstructionScript)

(fn GetClosestTarget
  (params (List :type Array%20of%20Actor%20Object%20References))
  (for _array_element List
    (LocalVariables|GetTempTarget
      (:then
        (if (< (LocalVariables|GetTempDistance) (Math|Vector|VectorLength (- (Transformation|GetActorLocation) (Transformation|GetActorLocation _array_element))))
          (LocalVariables|SetTempTarget _array_element)
          (LocalVariables|SetTempDistance (Math|Vector|VectorLength (- (Transformation|GetActorLocation) (Transformation|GetActorLocation _array_element))))))
      (:else
        (LocalVariables|SetTempTarget _array_element)
        (LocalVariables|SetTempDistance (Math|Vector|VectorLength (- (Transformation|GetActorLocation) (Transformation|GetActorLocation _array_element)))))))
  (return (LocalVariables|GetTempTarget)))