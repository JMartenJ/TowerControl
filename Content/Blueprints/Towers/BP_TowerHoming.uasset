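; Tower-defense tower that fires homing projectiles at overlapping enemies, with LowFireRate and RapidFire variants selected by TypeOfTower.
; BeginPlay loads the variant's TowerData row to set mesh, range sphere radius and looping fire timer.
; Each tick of that timer spawns BP_ProjectileHoming at the enemy returned by GetClosestTarget.
; Despite its name, GetClosestTarget's comparison keeps the farthest enemy.
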(event Custom|FireRapid
  ;[1 1 1] RapidFire
  (bind _targets (CallFunction|GetClosestTarget (Collision|GetOverlappingActors "/Game/Blueprints/Enemies/BP_EnemyMaster.BP_EnemyMaster_C" :!class /Script/Engine.Actor)))
  (bind _asbp_enemy_master (Utilities|Casting|CastToBP_EnemyMaster _targets))
  (Game|SpawnActorfromClass "/Game/Blueprints/Towers/BP_ProjectileHoming.BP_ProjectileHoming_C" (Transformation|GetActorTransform) "AlwaysSpawn" 0 _asbp_enemy_master 0))

(event Custom|InitRapidFire
  ;[1 1 1] RapidFire
  (if (Utilities|Name|Equal(Name) (Variables|Default|GetTypeOfTower) "RapidFire")
    (bind _returnvalue (Utilities|GetDataTableRow "/Game/Blueprints/TowerData.TowerData" "RapidFire")
      (:then
        (Components|StaticMesh|SetStaticMesh (Variables|Default|GetTowerMesh) (.mesh _returnvalue))
        (Components|Sphere|SetSphereRadius (Variables|Default|GetSphere) (.range _returnvalue) true)
        (Utilities|Time|SetTimerbyFunctionName 0 "FireRapid" (.firerate _returnvalue) true)))))

(event Custom|FireHoming
  ;[1 1 1] LowFireRate
  (bind _targets (CallFunction|GetClosestTarget (Collision|GetOverlappingActors "/Game/Blueprints/Enemies/BP_EnemyMaster.BP_EnemyMaster_C" :!class /Script/Engine.Actor)))
  (bind _asbp_enemy_master (Utilities|Casting|CastToBP_EnemyMaster _targets))
  (Game|SpawnActorfromClass "/Game/Blueprints/Towers/BP_ProjectileHoming.BP_ProjectileHoming_C" (Transformation|GetActorTransform) "AlwaysSpawn" 0 _asbp_enemy_master 0))

(event Custom|InitLowFireRate
  ;[1 1 1] LowFireRate
  (if (Utilities|Name|Equal(Name) (Variables|Default|GetTypeOfTower) "LowFireRate")
    (bind _returnvalue (Utilities|GetDataTableRow "/Game/Blueprints/TowerData.TowerData" "LowFireRate")
      (:then
        (Components|StaticMesh|SetStaticMesh (Variables|Default|GetTowerMesh) (.mesh _returnvalue))
        (Components|Sphere|SetSphereRadius (Variables|Default|GetSphere) (.range _returnvalue) true)
        (Utilities|Time|SetTimerbyFunctionName 0 "FireHoming" (.firerate _returnvalue) true)))))

(event EventBeginPlay
  (Utilities|FlowControl|Sequence
    (:then_0
      (CallFunction|InitLowFireRate))
    (:then_1
      (CallFunction|InitRapidFire))))

(fn ConstructionScript)

(fn GetClosestTarget
  (params (List :type Array%20of%20Actor%20Object%20References))
  (for _array_element List
    (LocalVariables|GetTempTarget
      (:then
        (if (< (LocalVariables|GetTempDistance) (Math|Vector|VectorLength (- (Transformation|GetActorLocation) (Transformation|GetActorLocation _array_element))))
          (LocalVariables|SetTempTarget _array_element)
          (LocalVariables|SetTempDistance (Math|Vector|VectorLength (- (Transformation|GetActorLocation) (Transformation|GetActorLocation _array_element))))))
      (:else
        (LocalVariables|SetTempTarget _array_element)
        (LocalVariables|SetTempDistance (Math|Vector|VectorLength (- (Transformation|GetActorLocation) (Transformation|GetActorLocation _array_element)))))))
  (return (LocalVariables|GetTempTarget)))