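; Basic tower projectile that deals one point of damage to an enemy.
; On BeginPlay it stores the target enemy's location, then moves toward that fixed point at constant speed each Tick, without homing.
; Overlapping any BP_EnemyMaster subtracts health, destroys the projectile and calls that enemy's CheckIsDead.
; A Delay in Tick destroys the projectile after about three seconds if it hits nothing.
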(event Collision|EventActorBeginOverlap
  (params (OtherActor :type Actor%20Object%20Reference))
  (bind _asbp_enemy_master (Utilities|Casting|CastToBP_EnemyMaster OtherActor))
  (Variables|/Game/Blueprints/Enemies/BP_EnemyMaster.BP_EnemyMaster_C|SetHealth _asbp_enemy_master (- (Variables|/Game/Blueprints/Enemies/BP_EnemyMaster.BP_EnemyMaster_C|GetHealth _asbp_enemy_master) 1.0))
  (Actor|DestroyActor)
  (Default|CheckIsDead _asbp_enemy_master))

(event EventBeginPlay
  (Variables|Default|SetLastKnownLocation (Transformation|GetActorLocation (Variables|Default|GetTargetEnemy))))

(event EventTick
  (params (DeltaSeconds :type Float%20%28single-precision%29))
  (Transformation|SetActorLocation (Math|Interpolation|VInterptoConstant (Transformation|GetActorLocation) (Variables|Default|GetLastKnownLocation) DeltaSeconds (Variables|Default|GetProjectileSpeed)) false false)
  (Utilities|FlowControl|Delay 3.0)
  (Actor|DestroyActor))

(fn ConstructionScript)