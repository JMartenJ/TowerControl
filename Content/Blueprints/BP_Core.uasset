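; BP_Core is a destructible core actor that loses health once an actor tagged "enemy" overlaps it.
; The overlap starts a looping one-second timer, with no clear on overlap end, that calls ChangeHealth and IsDead on the HUD widget.
; The core creates that Widget_HUD on BeginPlay and reads CoreHealth from it, destroying itself when the value reaches zero.
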(event Custom|DestroyCore
  (Default|ChangeHealth (stale EventBeginPlay _output_get))
  (Default|IsDead? (stale EventBeginPlay _output_get))
  (if (== (Variables|/Game/Interface/Widget_HUD.Widget_HUD_C|GetCoreHealth (stale EventBeginPlay _output_get)) 0)
    (Actor|DestroyActor)))

(event EventBeginPlay
  (bind _returnvalue (UserInterface|CreateWidget "/Game/Interface/Widget_HUD.Widget_HUD_C"))
  (bind _output_get (Variables|Default|SetWidgetReference _returnvalue))
  (UserInterface|Viewport|AddtoViewport _output_get 0))

(event Collision|EventActorBeginOverlap
  (params (OtherActor :type Actor%20Object%20Reference))
  (if (Actor|ActorHasTag OtherActor "enemy")
    (Utilities|Time|SetTimerbyEvent (delegate Custom|DestroyCore) 1.0 true)))

(fn ConstructionScript)